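; BP_Dome is an actor whose Sphere component grows smoothly when its Expand event is called with an amount.
; Expand captures the current X scale, then a timeline lerps a uniform world scale from that value to that value plus the amount.
; The timeline plays at half rate for expansions above a fixed threshold, so larger growth takes longer.
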(event Custom|Expand
  (params (ExpandAmount :type Float%20%28single-precision%29))
  (bind _output_get (Variables|Default|SetCurrentExpandAmount ExpandAmount))
  (Variables|Default|SetTempScale (.x (Variables|/Script/Engine.SceneComponent|GetRelativeScale3D (Variables|Default|GetSphere))))
  (Components|Timeline|SetPlayRate (Variables|Default|GetTimeline_0) (select (<= _output_get 1e+01) 1.0 0.5))
  (bind _newtrack_0 (Timeline|Timeline_0 PlayFromStart)
    (:Update
      (Transformation|SetWorldScale3D (Variables|Default|GetSphere) (Math|Vector|MakeVector (Math|Float|Lerp (Variables|Default|GetTempScale) (+ (Variables|Default|GetTempScale) (Variables|Default|GetCurrentExpandAmount)) _newtrack_0) (Math|Float|Lerp (Variables|Default|GetTempScale) (+ (Variables|Default|GetTempScale) (Variables|Default|GetCurrentExpandAmount)) _newtrack_0) (Math|Float|Lerp (Variables|Default|GetTempScale) (+ (Variables|Default|GetTempScale) (Variables|Default|GetCurrentExpandAmount)) _newtrack_0))))))

(event EventBeginPlay)

(fn ConstructionScript)